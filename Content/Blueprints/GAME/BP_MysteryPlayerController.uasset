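; BP_MysteryPlayerController is the player controller for the mystery game, handling input setup and camera look.
; On BeginPlay it switches to game-only input, hides the mouse cursor and adds the IMC_MysteryGame Enhanced Input mapping context.
; The IA_Look action feeds yaw and inverted pitch input to rotate the view.
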(event `self.ReceiveBeginPlay`
  (bind _returnvalue (pcsubsystem `EnhancedInputLocalPlayerSubsystem` self))
  (`|ExecutionSequence`
    (:`then_0`
      ;[1 0.1506 0.4777] might have to change this later
      (`WidgetBlueprintLibrary.SetInputMode_GameOnly` self)
      (set `self.bShowMouseCursor` false)
      (`/Engine/EditorBlueprintResources/StandardMacros.IsValid` _returnvalue
        (:`Is Valid`
          (`EnhancedInputSubsystemInterface.AddMappingContext` _returnvalue "/Game/Blueprints/Inputs/IMC_MysteryGame.IMC_MysteryGame" 0 (struct)))))))

(event `EnhancedInput|/Game/Blueprints/Inputs/Actions/IA_Look`
  (params (ActionValue :type "Vector2D Structure") (ElapsedSeconds :type "Float (double-precision)") (TriggeredSeconds :type "Float (double-precision)") (InputAction :type "InputAction Object Reference" :default "/Game/Blueprints/Inputs/Actions/IA_Look.IA_Look"))
  (:`Triggered`
    (`self.AddYawInput` ActionValue_X)
    (`self.AddPitchInput` (* ActionValue_Y -1.0))))

(fn `UserConstructionScript`)